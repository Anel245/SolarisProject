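; BP_NextLevel is a level-exit trigger actor that shows the win screen once every enemy is dead.
; When a PlayerCharacter overlaps its Box, it checks whether EnemiesAlive on SolarisGameMode is zero.
; If so, it adds the WBP_Win widget to the viewport and disables the player's movement and input.
; It does not load another level itself, despite its name.
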(event OnComponentBeginOverlap(Box)
  (params (OverlappedComponent :type Primitive%20Component%20Object%20Reference) (OtherActor :type Actor%20Object%20Reference) (OtherComp :type Primitive%20Component%20Object%20Reference) (OtherBodyIndex :type Integer) (bFromSweep :type Boolean) (SweepResult :type Hit%20Result%20Structure%20%28by%20ref%29))
  (bind _asplayer_character (Utilities|Casting|CastToPlayerCharacter OtherActor))
  (bind _assolaris_game_mode (Utilities|Casting|CastToSolarisGameMode (Game|GetGameMode)))
  (if (== (Variables|/Game/Devs/Mert/Blueprints/Player/Input/SolarisGameMode.SolarisGameMode_C|GetEnemies%20Alive _assolaris_game_mode) 0)
    (bind _returnvalue (UserInterface|CreateWidget "/Game/Devs/Mert/Blueprints/Player/Widgets/WBP_Win.WBP_Win_C"))
    (UserInterface|Viewport|AddtoViewport _returnvalue 0)
    (Pawn|Components|CharacterMovement|DisableMovement (Variables|/Script/Engine.Character|GetCharacterMovement _asplayer_character))
    (Input|DisableInput _asplayer_character 0)))

(event EventBeginPlay)

(event Collision|EventActorBeginOverlap
  (params (OtherActor :type Actor%20Object%20Reference)))

(event EventTick
  (params (DeltaSeconds :type Float%20%28single-precision%29)))

(fn ConstructionScript)